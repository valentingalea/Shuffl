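; Player-controller Blueprint that handles touch placement of the AR table during AR setup.
; While ARSetup is true, a touch press traces the touch position against AR tracked objects, with feature-point and ground-plane tests off.
; The first hit's transform spawns a BPC_HighQualityTable, which clears ARSetup and is stored as ARTable on the SceneProps actor.
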(event `InputTouch`
  (params (Location :type "Vector Structure") (FingerIndex :type "ETouchIndex Enum"))
  (bind (_locationx _locationy) (`self.GetInputTouchState` (`GameplayStatics.GetPlayerController` 0) "Touch1"))
  (:`Pressed`
    (if (`self.ARSetup`)
      (bind _returnvalue (`ARBlueprintLibrary.LineTraceTrackedObjects` (`KismetMathLibrary.MakeVector2D` _locationx _locationy) false false))
      (`/Engine/EditorBlueprintResources/StandardMacros.CompareInt` (`KismetArrayLibrary.Array_Length` _returnvalue)
        (:`>`
          (bind _returnvalue_2 (`|SpawnActorFromClass` "/Game/HighQualityTable/BPC_HighQualityTable.BPC_HighQualityTable_C" (`ARTraceResultLibrary.GetLocalToWorldTransform` (`|GetArrayItem` _returnvalue)) "Undefined" "OverrideRootScale" null null))
          (set `self.ARSetup` false)
          (bind _returnvalue_3 (`GameplayStatics.GetActorOfClass` "/Script/Shuffl.SceneProps"))
          (set `SceneProps.ARTable` _returnvalue_2 _returnvalue_3))))))

(fn `UserConstructionScript`)