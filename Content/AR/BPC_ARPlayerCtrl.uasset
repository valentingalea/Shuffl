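; AR player controller Blueprint for the Shuffl game that handles placing the table in the real world.
; While AR setup is active, a touch line-traces tracked AR geometry, ignoring feature points and the ground plane.
; The first hit moves and reveals the SceneProps AR table, ends setup and switches to detail view.
; The Quit input stops the AR session.
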(event `InputAction|Quit`
  (params (Key :type "Key Structure"))
  (:`Pressed`
    (`ARBlueprintLibrary.StopARSession`)))

(event `InputTouch`
  (params (Location :type "Vector Structure") (FingerIndex :type "ETouchIndex Enum"))
  (bind (_locationx _locationy) (`self.GetInputTouchState` (`GameSubSys.ShufflGetActivePlayerCtrl`) "Touch1"))
  (:`Pressed`
    (if (`self.ARSetup`)
      (bind _returnvalue (`ARBlueprintLibrary.LineTraceTrackedObjects` (`KismetMathLibrary.MakeVector2D` _locationx _locationy) false false))
      (`/Engine/EditorBlueprintResources/StandardMacros.CompareInt` (`KismetArrayLibrary.Array_Length` _returnvalue)
        (:`>`
          (bind _returnvalue_2 (`GameplayStatics.GetActorOfClass` "/Script/Shuffl.SceneProps"))
          (bind _artable (`SceneProps.ARTable` _returnvalue_2))
          (`self.K2_SetActorTransform` _artable (`ARTraceResultLibrary.GetLocalToWorldTransform` (`|GetArrayItem` _returnvalue)) false false)
          (`self.SetActorHiddenInGame` _artable false)
          (bind _asbpc_arplayer_ctrl (cast `/Game/AR/BPC_ARPlayerCtrl` (`GameSubSys.ShufflGetActivePlayerCtrl`)))
          (set `self.ARSetup` false)
          (`self.SwitchToDetailView` _asbpc_arplayer_ctrl))))))

(fn `UserConstructionScript`)